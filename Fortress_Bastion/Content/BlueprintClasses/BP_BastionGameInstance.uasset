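; Game instance that connects to a local WebSocket server at startup and handles player authentication.
; Init creates a WebSocketManager after a short delay and binds its connection, account and login events.
; On connection, it logs in with the first saved account's token, or shows UI_Login without a save.
; Account creation saves the token to a new save object and opens MainGame_Map, as does login success; login failure shows UI_Login.
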(event Custom|HandleOnConnected
  (Development|PrintString "Successfully connected to server!")
  (bind _returnvalue (SaveGame|DoesSaveGameExist "MainSaveSlot"))
  (if _returnvalue
    (bind _returnvalue_2 (SaveGame|LoadGamefromSlot "MainSaveSlot"))
    (bind _asbastion_save_game (Utilities|Casting|CastToBastionSaveGame _returnvalue_2))
    (Class|WebSocketManager|LoginwithToken (Variables|Default|GetWebSocketManager) (.Login (Utilities|Struct|BreakAccountData (Utilities|Array|Get(acopy) (Variables|/Script/Fortress_Bastion.BastionSaveGame|GetSavedAccounts _asbastion_save_game)))) (.AuthToken (Utilities|Struct|BreakAccountData (Utilities|Array|Get(acopy) (Variables|/Script/Fortress_Bastion.BastionSaveGame|GetSavedAccounts _asbastion_save_game)))))
    (else
      (bind _returnvalue_3 (UserInterface|CreateWidget "/Game/BlueprintWidget/UI_Login.UI_Login_C"))
      (UserInterface|Viewport|AddtoViewport _returnvalue_3 0))))

(event Custom|HandleConnectionError
  (params (ErrorMessage :type String))
  (Development|PrintString ErrorMessage))

(event Custom|HandleAccountCreated
  (params (PlayerID :type String) (PlayerName :type String) (Token :type String))
  (bind _returnvalue (SaveGame|CreateSaveGameObject "/Game/BlueprintClasses/BP_BastionSaveGame.BP_BastionSaveGame_C"))
  (bind _returnvalue_2 (Utilities|Array|Add (Variables|/Script/Fortress_Bastion.BastionSaveGame|GetSavedAccounts _returnvalue) (Utilities|Struct|MakeAccountData PlayerID Token)))
  (SaveGame|SaveGametoSlot _returnvalue "MainSaveSlot" _returnvalue_2)
  (Game|OpenLevel(byName) "MainGame_Map"))

(event Custom|HandleLoginSuccess
  (Development|PrintString "Login successful! Opening level...")
  (Game|OpenLevel(byName) "MainGame_Map")
  (Development|PrintString "HelloWorld"))

(event Custom|HandleLoginFailed
  (params (ErrorMessage :type String))
  (bind _returnvalue (UserInterface|CreateWidget "/Game/BlueprintWidget/UI_Login.UI_Login_C"))
  (UserInterface|Viewport|AddtoViewport _returnvalue 0))

(event EventInit
  (bind _websocketmanager (Variables|Default|GetWebSocketManager))
  (Utilities|FlowControl|Delay 0.2)
  (Game|ConstructObjectfromClass "/Script/Fortress_Bastion.WebSocketManager" "BP_BastionGameInstance")
  (Development|PrintString "start (OnConnected)")
  (EventDispatchers|AssignOnConnected _websocketmanager (delegate Custom|HandleOnConnected))
  (Development|PrintString "Ok>Sart (OnAccountCreated)")
  (EventDispatchers|BindEventtoOnAccountCreated _websocketmanager (delegate Custom|HandleAccountCreated))
  (Development|PrintString "Ok>Start (OnLoginSuccess)")
  (EventDispatchers|BindEventtoOnLoginSuccess _websocketmanager (delegate Custom|HandleLoginSuccess))
  (Development|PrintString "Ok>Start (OnLoginFailed)")
  (EventDispatchers|BindEventtoOnLoginFailed _websocketmanager (delegate Custom|HandleLoginFailed))
  (Development|PrintString "Ok>Start (Connected)")
  (EventDispatchers|BindEventtoOnConnectionError _websocketmanager (delegate Custom|HandleConnectionError))
  (Class|WebSocketManager|Connect _websocketmanager "ws://localhost:8080")
  (Development|PrintString "Attempting to connect..."))

(fn InitializeAuthorizationLogic)